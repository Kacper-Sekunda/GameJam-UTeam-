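; BP_Cursor is a world-space mouse cursor that shows context icons and forwards clicks to interactable actors.
; Each tick it projects the mouse ray onto a horizontal plane at fixed height, moves its W_Cursor widget there, and line-traces onward along that ray.
; Hit actors implementing BPI_CursorIcons supply the icon, otherwise the default is used.
; Click repeats the trace and sends ClickMessage to BPI_Interaction actors.
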(event `self.ReceiveBeginPlay`
  (bind _asw_cursor (cast `/Game/Blueprints/Character/Cursor/W_Cursor` (`WidgetComponent.GetWidget` (`self.Widget`))))
  (set `self.Cursor Icon Widget` _asw_cursor))

(event `self.ReceiveTick`
  (params (DeltaSeconds :type "Float (single-precision)"))
  (bind (_worldlocation _worlddirection) (`PlayerController.DeprojectMousePositionToWorld` (`GameplayStatics.GetPlayerController` 0)))
  (bind (_t _intersection) (`KismetMathLibrary.LinePlaneIntersection` _worldlocation (+ _worldlocation (* _worlddirection 15000.0)) (`KismetMathLibrary.MakePlaneFromPointAndNormal` (0.0 0.0 200.0) (0.0 0.0 1.0))))
  (`SceneComponent.K2_SetWorldLocation` (`self.Widget`) _intersection false false)
  (`self.Find Icon Line Trace` _intersection (+ _intersection (* _worlddirection 5000.0))))

(event `Click`
  (bind (_worldlocation _worlddirection) (`PlayerController.DeprojectMousePositionToWorld` (`GameplayStatics.GetPlayerController` 0)))
  (bind (_t _intersection) (`KismetMathLibrary.LinePlaneIntersection` _worldlocation (+ _worldlocation (* _worlddirection 15000.0)) (`KismetMathLibrary.MakePlaneFromPointAndNormal` (0.0 0.0 200.0) (0.0 0.0 1.0))))
  (`self.Click Line Trace` _intersection (+ _intersection (* _worlddirection 5000.0))))

(event `Set Icon`
  (params (Icon :type "PaperSprite Object Reference"))
  (`/Game/Blueprints/Character/Cursor/W_Cursor.Set Icon` (`self.Cursor Icon Widget`) Icon))

(fn `Click Line Trace`
  (params (Start :type "Vector Structure") (End :type "Vector Structure"))
  (bind _outhit (`KismetSystemLibrary.LineTraceSingle` :`Start` Start :`End` End :`TraceChannel` "TraceTypeQuery1" :`DrawDebugType` "ForOneFrame"))
  (if (`KismetSystemLibrary.DoesImplementInterface` (`.HitActor` (`GameplayStatics.BreakHitResult` _outhit)) "/Game/Blueprints/Character/Cursor/BPI_Interaction.BPI_Interaction_C")
    (message `/Game/Blueprints/Character/Cursor/BPI_Interaction.Click` (`.HitActor` (`GameplayStatics.BreakHitResult` _outhit)))))

(fn `Find Icon Line Trace`
  (params (Start :type "Vector Structure") (End :type "Vector Structure"))
  (bind _outhit (`KismetSystemLibrary.LineTraceSingle` :`Start` Start :`End` End :`TraceChannel` "TraceTypeQuery1" :`DrawDebugType` "ForOneFrame"))
  (`KismetSystemLibrary.PrintString` (`KismetSystemLibrary.GetDisplayName` (`.HitComponent` (`GameplayStatics.BreakHitResult` _outhit))))
  (if (`KismetSystemLibrary.DoesImplementInterface` (`.HitActor` (`GameplayStatics.BreakHitResult` _outhit)) "/Game/Blueprints/Character/Cursor/BPI_CursorIcons.BPI_CursorIcons_C")
    (bind _icon (message `/Game/Blueprints/Character/Cursor/BPI_CursorIcons.Find Icon` (`.HitActor` (`GameplayStatics.BreakHitResult` _outhit)) (`.HitComponent` (`GameplayStatics.BreakHitResult` _outhit))))
    (if (== _icon null)
      (`/Game/Blueprints/Character/Cursor/W_Cursor.Set Icon` (`self.Cursor Icon Widget`) (`self.Default Cursor Icon`) :!label _label)
      (else
        (`/Game/Blueprints/Character/Cursor/W_Cursor.Set Icon` (`self.Cursor Icon Widget`) _icon)))
    (else
      (goto _label))))

(fn `UserConstructionScript`)