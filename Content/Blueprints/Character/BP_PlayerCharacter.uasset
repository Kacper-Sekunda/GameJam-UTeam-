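; Player character that acts as a fixed-viewpoint camera, gliding between placed BP_CameraPoint actors such as desk, X-ray, sucker and conveyor end.
; Holding a look-at input moves to its point and releasing returns to the default view, with ActiveHeldKey blocking other inputs meanwhile.
; A timeline lerps actor location and camera rotation from their current values toward the cached target each update.
; An idle camera shake starts on BeginPlay.
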(event `self.ReceiveBeginPlay`
  (`KismetSystemLibrary.Delay` 0.01)
  (bind _outactors (`GameplayStatics.GetAllActorsOfClass` "/Game/Blueprints/Character/Camera/BP_CameraPoint.BP_CameraPoint_C"))
  (set `self.FocusPoints` _outactors)
  (bind (_location _rotation) (`self.GetCameraFocusTransform` "NewEnumerator2"))
  (`self.SetFocusLocationAndRotation` _location _rotation)
  (`PlayerController.ClientStartCameraShake` :`self` (`GameplayStatics.GetPlayerController` 0) :`Shake` "/Game/Blueprints/Idle.Idle_C"))

(event `Key|S`
  (params (Key :type "Key Structure")))

(event `EnhancedInput|/Game/Blueprints/Inputs/Input_Actions/IA_LookAtDesk`
  (params (ActionValue :type Boolean) (ElapsedSeconds :type "Float (double-precision)") (TriggeredSeconds :type "Float (double-precision)") (InputAction :type "InputAction Object Reference" :default "/Game/Blueprints/Inputs/Input_Actions/IA_LookAtDesk.IA_LookAtDesk"))
  (bind _active_held_key (`self.Active Held Key`))
  (:`Triggered`
    (if (`|EnumEquality` _active_held_key "NewEnumerator0")
      (set `self.Active Held Key` "NewEnumerator1")
      (`self.Set Target Focus Point` "NewEnumerator1")
      (`self.Move To Target`)))
  (:`Completed`
    (if (`|EnumEquality` _active_held_key "NewEnumerator1")
      (set `self.Active Held Key` "NewEnumerator0")
      (`self.Set Target Focus Point` "NewEnumerator2" :!label _label)
      (`self.Move To Target`))))

(event `EnhancedInput|/Game/Blueprints/Inputs/Input_Actions/IA_LookAtXray`
  (params (ActionValue :type Boolean) (ElapsedSeconds :type "Float (double-precision)") (TriggeredSeconds :type "Float (double-precision)") (InputAction :type "InputAction Object Reference" :default "/Game/Blueprints/Inputs/Input_Actions/IA_LookAtXray.IA_LookAtXray"))
  (bind _active_held_key (`self.Active Held Key`))
  (:`Triggered`
    (if (`|EnumEquality` _active_held_key "NewEnumerator0")
      (set `self.Active Held Key` "NewEnumerator4")
      (`self.Set Target Focus Point` "NewEnumerator4")
      (`self.Move To Target`)))
  (:`Completed`
    (if (`|EnumEquality` _active_held_key "NewEnumerator4")
      (set `self.Active Held Key` "NewEnumerator0")
      (goto _label))))

(event `EnhancedInput|/Game/Blueprints/Inputs/Input_Actions/IA_LookAtSucker`
  (params (ActionValue :type Boolean) (ElapsedSeconds :type "Float (double-precision)") (TriggeredSeconds :type "Float (double-precision)") (InputAction :type "InputAction Object Reference" :default "/Game/Blueprints/Inputs/Input_Actions/IA_LookAtSucker.IA_LookAtSucker"))
  (bind _active_held_key (`self.Active Held Key`))
  (:`Triggered`
    (if (`|EnumEquality` _active_held_key "NewEnumerator0")
      (set `self.Active Held Key` "NewEnumerator5")
      (`self.Set Target Focus Point` "NewEnumerator5")
      (`self.Move To Target`)))
  (:`Completed`
    (if (`|EnumEquality` _active_held_key "NewEnumerator5")
      (set `self.Active Held Key` "NewEnumerator0")
      (goto _label))))

(event `EnhancedInput|/Game/Blueprints/Inputs/Input_Actions/IA_LookAtConveyerEnd`
  (params (ActionValue :type Boolean) (ElapsedSeconds :type "Float (double-precision)") (TriggeredSeconds :type "Float (double-precision)") (InputAction :type "InputAction Object Reference" :default "/Game/Blueprints/Inputs/Input_Actions/IA_LookAtConveyerEnd.IA_LookAtConveyerEnd"))
  (bind _active_held_key (`self.Active Held Key`))
  (:`Triggered`
    (if (`|EnumEquality` _active_held_key "NewEnumerator0")
      (set `self.Active Held Key` "NewEnumerator6")
      (`self.Set Target Focus Point` "NewEnumerator6")
      (`self.Move To Target`)))
  (:`Completed`
    (if (`|EnumEquality` _active_held_key "NewEnumerator6")
      (set `self.Active Held Key` "NewEnumerator0")
      (goto _label))))

(event `Move To Target`
  (bind (_target_transform_location _target_transform_rotation) (`KismetMathLibrary.BreakTransform` (`self.Target Transform`)))
  (bind (_direction _alpha) (`Timeline|Timeline_2` :!via `PlayFromStart`)
    (:`Update`
      (bind (_location _rotation) (`self.Lerp` _target_transform_location _target_transform_rotation _alpha))
      (`self.SetFocusLocationAndRotation` _location _rotation))))

(fn `GetCameraFocusTransform`
  (params (`Focus Point` :type "/Game/Blueprints/Character/Camera/E_CameraFocus Enum" :default "NewEnumerator0"))
  (returns (Location :type "Vector Structure") (Rotation :type "Rotator Structure"))
  (for _array_element (`self.FocusPoints`)
    (if (`|EnumEquality` (`/Game/Blueprints/Character/Camera/BP_CameraPoint.CameraFocusPoint` _array_element) `Focus Point`)
      (bind (_returnvalue_location _returnvalue_rotation) (`KismetMathLibrary.BreakTransform` (`self.GetTransform` _array_element)))
      (return _returnvalue_location _returnvalue_rotation))))

(fn `Lerp`
  (params (NewLocation :type "Vector Structure") (NewRotation :type "Rotator Structure") (Alpha :type "Float (double-precision)"))
  (returns (Location :type "Vector Structure") (Rotation :type "Rotator Structure"))
  (return (`KismetMathLibrary.VLerp` (`self.K2_GetActorLocation`) NewLocation Alpha) (`KismetMathLibrary.RLerp` (`SceneComponent.K2_GetComponentRotation` (`self.Camera`)) NewRotation Alpha true)))

(fn `Set Target Focus Point`
  (params (`New Target Focus Point` :type "/Game/Blueprints/Character/Camera/E_CameraFocus Enum" :default "NewEnumerator0"))
  (bind (_location _rotation) (`self.GetCameraFocusTransform` `New Target Focus Point`))
  (set `self.Target Transform` (`KismetMathLibrary.MakeTransform` _location _rotation)))

(fn `SetFocusLocationAndRotation`
  (params (Location :type "Vector Structure") (Rotation :type "Rotator Structure"))
  (`self.K2_SetActorLocation` Location)
  (`SceneComponent.K2_SetWorldRotation` (`self.Camera`) Rotation false false))

(fn `UserConstructionScript`)