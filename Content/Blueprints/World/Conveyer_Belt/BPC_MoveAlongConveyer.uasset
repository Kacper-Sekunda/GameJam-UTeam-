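; BPC_MoveAlongConveyer is an actor component that moves its owner along a conveyor belt's spline.
; On BeginPlay it caches the first BP_ConveyerBelt found in the world.
; While active, Tick advances a distance by the belt's speed and sets the owner's transform to that point on the spline, without sweeping.
; TurnOn, TurnOff and SetDistance events control movement and position along the belt.
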(event `self.ReceiveBeginPlay`
  (bind _returnvalue (`GameplayStatics.GetActorOfClass` "/Game/Blueprints/World/Conveyer_Belt/BP_ConveyerBelt.BP_ConveyerBelt_C"))
  (`/Engine/EditorBlueprintResources/StandardMacros.IsValid` _returnvalue
    (:`Is Valid`
      (set `self.Conveyer` _returnvalue))))

(event `self.ReceiveTick`
  (params (DeltaSeconds :type "Float (single-precision)"))
  (if (`self.Active`)
    (bind _output_get (set `self.Current Distance` (+ (`self.Current Distance`) (* (`/Game/Blueprints/World/Conveyer_Belt/BP_ConveyerBelt.Speed` (`self.Conveyer`)) DeltaSeconds))))
    (`Actor.K2_SetActorTransform` (`self.GetOwner`) (`SplineComponent.GetTransformAtDistanceAlongSpline` (`/Game/Blueprints/World/Conveyer_Belt/BP_ConveyerBelt.Spline` (`self.Conveyer`)) _output_get "World" false) false false)))

(event `Turn On`
  (set `self.Active` true))

(event `Turn Off`
  (set `self.Active` false))

(event `Set Distance`
  (params (`New Distance` :type "Float (double-precision)"))
  (set `self.Current Distance` `New Distance`))