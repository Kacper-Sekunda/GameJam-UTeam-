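; Base clickable box that travels on the BP_ConveyerBelt, holds a child-actor object, and can be pulled onto a BP_Sucker anchor to open or close.
; Clicking swaps it between belt and anchor; returning searches forward along the spline for an overlap-free spot.
; Tick drives timeline-eased lerps that track the moving belt, then hands off to BPCMoveAlongConveyer.
; Collision toggles gate body and flap clicks, with cursor icons from BPCCursorIcon.
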(event `self.ReceiveBeginPlay`
  (`/Game/Blueprints/Character/Cursor/BPC_CursorIcon.Create New Icon` (`self.BPC_CursorIcon`) "/Game/Assets/Images/GrabHandCursor_Sprite.GrabHandCursor_Sprite" (`|MakeArray` null (`self.untitled`) null :!type "SceneComponent Object Reference"))
  (`/Game/Blueprints/Character/Cursor/BPC_CursorIcon.Create New Icon` (`self.BPC_CursorIcon`) "/Game/Assets/Images/Craft_Knife_Sprite.Craft_Knife_Sprite" (`|MakeArray` (`self.Cube`) :!type "SceneComponent Object Reference"))
  (`/Game/Blueprints/Character/Cursor/BPC_CursorIcon.Create New Icon` (`self.BPC_CursorIcon`) "/Game/Assets/Images/Craft_Knife_Sprite.Craft_Knife_Sprite" (`SceneComponent.GetChildrenComponents` (`self.Flaps`) false))
  (bind _returnvalue (`GameplayStatics.GetActorOfClass` "/Game/Blueprints/World/Conveyer_Belt/BP_ConveyerBelt.BP_ConveyerBelt_C"))
  (set `self.Conveyer Belt` _returnvalue)
  (bind _returnvalue_2 (`GameplayStatics.GetActorOfClass` "/Game/Blueprints/World/Sucker/BP_Sucker.BP_Sucker_C"))
  (set `self.Anchor` _returnvalue_2)
  (`ChildActorComponent.SetChildActorClass` (`self.Object`) (`self.Object Class`))
  (`self.Close`)
  (`self.Update Collision`))

(event `self.ReceiveTick`
  (params (DeltaSeconds :type "Float (single-precision)"))
  (bind _returnvalue (+ (`self.Target Distance`) (* (`/Game/Blueprints/World/Conveyer_Belt/BP_ConveyerBelt.Speed` (`self.Conveyer Belt`)) (`GameplayStatics.GetWorldDeltaSeconds`))))
  (bind (_returnvalue_location _returnvalue_rotation) (`KismetMathLibrary.BreakTransform` (`SplineComponent.GetTransformAtDistanceAlongSpline` (`/Game/Blueprints/World/Conveyer_Belt/BP_ConveyerBelt.Spline` (`self.Conveyer Belt`)) _returnvalue "World" false)))
  (if (`self.Moving?`)
    (if (`self.Update Move With Conveyer?`)
      (set `self.Target Distance` _returnvalue)
      (`self.Set New Move Target` _returnvalue_location _returnvalue_rotation (- (`self.Move Time`) (`self.Current Move Time`)))
      (`self.Movement`)
      (else
        (`self.Movement`)))))

(event `/Game/Blueprints/Character/Cursor/BPI_Interaction.Click`
  (params (Object :type "ActorComponent Object Reference"))
  (bind _anchor (`self.Anchor`))
  (bind _anchor_2 (`self.Anchor`))
  (bind (_returnvalue_location _returnvalue_rotation) (`KismetMathLibrary.BreakTransform` (`self.GetTransform` _anchor_2)))
  (if (`self.Moving?`)
    _
    (elif (== Object (`self.untitled`))
      (if (`self.On Conveyer?`)
        (bind _ready_ (`/Game/Blueprints/World/Sucker/BP_Sucker.Ready To Receive?` _anchor))
        (if _ready_
          (`/Game/Blueprints/World/Sucker/BP_Sucker.Fill` _anchor_2 self)
          (`self.Set New Move Target` _returnvalue_location _returnvalue_rotation 1.0)
          (set `self.On Conveyer?` false))
        (else
          (bind _permission_ (`/Game/Blueprints/World/Sucker/BP_Sucker.Can I leave?` _anchor))
          (if _permission_
            (bind _target_distance (`self.Find Closest Legal Spline Point` (`/Game/Blueprints/World/Conveyer_Belt/BP_ConveyerBelt.Spline` (`self.Conveyer Belt`))))
            (set `self.Target Distance` _target_distance)
            (set `self.On Conveyer?` true)
            (`/Game/Blueprints/World/Sucker/BP_Sucker.Empty` (`self.Anchor`))
            (set `self.Update Move With Conveyer?` true)
            (if (not (`self.Closed?`))
              (`self.Close`)))))
      (elif (`self.On Conveyer?`)
        _
        (elif (== Object (`self.Cube`))
          (`self.Open`)
          (elif (== Object (`self.Cube1`))
            (`self.Close` :!label _label)
            (elif (== Object (`self.Cube2`))
              (goto _label))))))))

(event `Update Collision`
  (if (`self.On Conveyer?`)
    (`self.Disable Collision`)
    (elif (`self.Closed?`)
      (`PrimitiveComponent.SetCollisionEnabled` (`self.Cube`) "QueryAndPhysics")
      (`PrimitiveComponent.SetCollisionEnabled` (`self.Cube1`) "NoCollision")
      (`PrimitiveComponent.SetCollisionEnabled` (`self.Cube2`) "NoCollision")
      (else
        (`PrimitiveComponent.SetCollisionEnabled` (`self.Cube`) "NoCollision")
        (`PrimitiveComponent.SetCollisionEnabled` (`self.Cube1`) "QueryAndPhysics")
        (`PrimitiveComponent.SetCollisionEnabled` (`self.Cube2`) "QueryAndPhysics")))))

(event `Open`
  (`SkeletalMeshComponent.PlayAnimation` (`self.untitled`) "/Game/Assets/StaticMehes/BoxV3/Box_Opening.Box_Opening" false)
  (set `self.Closed?` false)
  (`self.Disable Collision`)
  (`KismetSystemLibrary.Delay` 1.0)
  (`self.Update Collision`))

(event `Close`
  (`SkeletalMeshComponent.PlayAnimation` (`self.untitled`) "/Game/Assets/StaticMehes/BoxV3/Box_Closing.Box_Closing" false)
  (set `self.Closed?` true)
  (`self.Disable Collision`)
  (`KismetSystemLibrary.Delay` 1.0)
  (`self.Update Collision`))

(event `Disable Collision`
  (`PrimitiveComponent.SetCollisionEnabled` (`self.Cube`) "NoCollision")
  (`PrimitiveComponent.SetCollisionEnabled` (`self.Cube1`) "NoCollision")
  (`PrimitiveComponent.SetCollisionEnabled` (`self.Cube2`) "NoCollision"))

(event `Set New Move Target`
  (params (Location :type "Vector Structure") (Rotation :type "Rotator Structure") (Time :type "Float (double-precision)"))
  (bind (_returnvalue_location _returnvalue_rotation _returnvalue_scale) (`KismetMathLibrary.BreakTransform` (`self.GetTransform`)))
  (`/Engine/EditorBlueprintResources/StandardMacros.CompareFloat` Time
    (:`>`
      (set `self.Move Time` Time)
      (set `self.Current Move Time` 0.0)
      (set `self.Recorded Transform` (`KismetMathLibrary.MakeTransform` _returnvalue_location _returnvalue_rotation _returnvalue_scale))
      (set `self.Target Transform` (`KismetMathLibrary.MakeTransform` Location Rotation _returnvalue_scale))
      (set `self.Moving?` true)
      (`/Game/Blueprints/World/Conveyer_Belt/BPC_MoveAlongConveyer.Turn Off` (`self.BPC_MoveAlongConveyer`)))
    (:`==`
      (`self.K2_SetActorTransform` (`KismetMathLibrary.MakeTransform` Location Rotation _returnvalue_scale) :!label _label_2)
      (set `self.Moving?` false)
      (set `self.Update Move With Conveyer?` false))
    (:`<`
      (goto _label_2))))

(event `Movement`
  (bind (_recorded_transform_location _recorded_transform_rotation _recorded_transform_scale) (`KismetMathLibrary.BreakTransform` (`self.Recorded Transform`)))
  (bind (_target_transform_location _target_transform_rotation) (`KismetMathLibrary.BreakTransform` (`self.Target Transform`)))
  (bind _returnvalue (+ (`self.Current Move Time`) (`GameplayStatics.GetWorldDeltaSeconds`)))
  (if (`self.Moving?`)
    (`/Engine/EditorBlueprintResources/StandardMacros.CompareFloat` _returnvalue (`self.Move Time`)
      (:`>`
        (set `self.Current Move Time` 1.0 :!label _label_3)
        (bind (_direction _newtrack_0) (`Timeline|Timeline` :`NewTime` (/ (`self.Current Move Time`) (`self.Move Time`)) :!via `SetNewTime` :!label _label_4)
          (:`Update`
            (`/Engine/EditorBlueprintResources/StandardMacros.CompareFloat` _newtrack_0 1.0
              (:`>`
                (set `self.Moving?` false :!label _label_5)
                (if (`self.On Conveyer?`)
                  (bind _returnvalue_2 (`KismetMathLibrary.VLerp` _recorded_transform_location _target_transform_location _newtrack_0))
                  (bind _returnvalue_3 (`KismetMathLibrary.RLerp` _recorded_transform_rotation _target_transform_rotation _newtrack_0))
                  (`self.K2_SetActorTransform` (`KismetMathLibrary.MakeTransform` _returnvalue_2 _returnvalue_3 _recorded_transform_scale))
                  (`/Game/Blueprints/World/Conveyer_Belt/BPC_MoveAlongConveyer.Set Distance` (`self.BPC_MoveAlongConveyer`) (`SplineComponent.GetDistanceAlongSplineAtLocation` (`/Game/Blueprints/World/Conveyer_Belt/BP_ConveyerBelt.Spline` (`self.Conveyer Belt`)) _returnvalue_2 "World"))
                  (`/Game/Blueprints/World/Conveyer_Belt/BPC_MoveAlongConveyer.Turn On` (`self.BPC_MoveAlongConveyer`))
                  (set `self.Update Move With Conveyer?` false)
                  (`self.Update Collision`)
                  (else
                    (`self.K2_SetActorTransform` (`KismetMathLibrary.MakeTransform` _returnvalue_2 _returnvalue_3 _recorded_transform_scale) :!label _label_6)
                    (`self.Update Collision`))))
              (:`==`
                (goto _label_5))
              (:`<`
                (goto _label_6))))))
      (:`==`
        (goto _label_3))
      (:`<`
        (set `self.Current Move Time` _returnvalue)
        (goto _label_4 :!via `SetNewTime`)))))

(fn `Check Box On Conveyer`
  (params (`Point to Check` :type "Vector Structure"))
  (returns (`Clear?` :type Boolean))
  (bind (_boxextent_x _boxextent_y _boxextent_z) (`KismetMathLibrary.BreakVector` (`BoxComponent.BoxExtent` (`self.Box`))))
  (bind (_outactors _returnvalue) (`KismetSystemLibrary.BoxOverlapActors` (`KismetMathLibrary.MakeVector` `Point to Check_X` `Point to Check_Y` (+ `Point to Check_Z` (/ _boxextent_z 2.0))) (`KismetMathLibrary.MakeVector` _boxextent_x _boxextent_y _boxextent_z) (`|MakeArray` "ObjectTypeQuery1" "ObjectTypeQuery2" "ObjectTypeQuery3" "ObjectTypeQuery4" "ObjectTypeQuery5" "ObjectTypeQuery6" :!type "EObjectTypeQuery Enum") "BP_BoxBase_C" (`|MakeArray` self :!type "Actor Object Reference")))
  (if _returnvalue
    (return false)
    (else
      (return true))))

(fn `Find Closest Legal Spline Point`
  (params (Spline :type "SplineComponent Object Reference"))
  (returns (`Target Distance` :type "Float (double-precision)"))
  (locals (`Starting Distance` :type "Float (double-precision)") (`Final Distance` :type "Float (double-precision)") (Variation :type "Float (double-precision)" :default 200.0) (`Current Distance` :type "Float (double-precision)"))
  (bind _output_get (set `local.Starting Distance` (`SplineComponent.GetDistanceAlongSplineAtLocation` Spline (`self.K2_GetActorLocation`) "World")))
  (set `local.Final Distance` (+ _output_get (`local.Variation`)))
  (bind (_returnvalue_location _returnvalue_rotation) (`KismetMathLibrary.BreakTransform` (`SplineComponent.GetTransformAtDistanceAlongSpline` Spline _output_get "World" false)))
  (bind _clear_ (`self.Check Box On Conveyer` _returnvalue_location))
  (if _clear_
    (`self.Set New Move Target` _returnvalue_location _returnvalue_rotation 1.0)
    (return _output_get)
    (else
      (set `local.Current Distance` (`local.Starting Distance`))
      (while (`KismetMathLibrary.BooleanNOR` (> (`local.Current Distance`) (`local.Final Distance`)) (== (`local.Current Distance`) (`local.Final Distance`)))
        (bind _output_get_2 (set `local.Current Distance` (+ (`local.Current Distance`) 5.0)))
        (bind (_returnvalue_location_2 _returnvalue_rotation_2) (`KismetMathLibrary.BreakTransform` (`SplineComponent.GetTransformAtDistanceAlongSpline` Spline _output_get_2 "World" false)))
        (bind _clear__2 (`self.Check Box On Conveyer` _returnvalue_location_2))
        (if _clear__2
          (`self.Set New Move Target` _returnvalue_location_2 _returnvalue_rotation_2 1.0)
          (return _output_get_2))))))

(fn `Find Icon`
  (params (Component :type "SceneComponent Object Reference"))
  (returns (Icon :type "PaperSprite Object Reference"))
  (bind _icon (`/Game/Blueprints/Character/Cursor/BPC_CursorIcon.Find Component Icon` (`self.BPC_CursorIcon`) Component))
  (return _icon))

(fn `Get Closest Point on Spline`
  (params (`Location To Check` :type "Vector Structure") (Spline :type "SplineComponent Object Reference"))
  (returns (ClosestPoint :type "Transform Structure"))
  (locals (Spline :type "SplineComponent Object Reference"))
  (bind _returnvalue (`SplineComponent.FindInputKeyClosestToWorldLocation` Spline `Location To Check`))
  (bind _returnvalue_2 (`KismetMathLibrary.FFloor` _returnvalue))
  (bind _returnvalue_3 (+ _returnvalue_2 1))
  (bind _returnvalue_4 (`SplineComponent.GetDistanceAlongSplineAtSplinePoint` Spline _returnvalue_3))
  (return (`SplineComponent.GetTransformAtDistanceAlongSpline` Spline (- _returnvalue_4 (* (- (`SplineComponent.GetDistanceAlongSplineAtSplinePoint` Spline _returnvalue_2) _returnvalue_4) (- _returnvalue _returnvalue_3))) "Local" false)))

(fn `Get Distance Along Spline Closest to Point`
  (params (`Location To Check` :type "Vector Structure") (Spline :type "SplineComponent Object Reference"))
  (returns (`Closest Distance` :type "Float (double-precision)"))
  (locals (Spline :type "SplineComponent Object Reference"))
  (bind _returnvalue (`SplineComponent.FindInputKeyClosestToWorldLocation` Spline `Location To Check`))
  (bind _returnvalue_2 (`KismetMathLibrary.FTrunc` _returnvalue))
  (bind _returnvalue_3 (`SplineComponent.GetDistanceAlongSplineAtSplinePoint` Spline _returnvalue_2))
  (return (+ _returnvalue_3 (* (- (`SplineComponent.GetDistanceAlongSplineAtSplinePoint` Spline (`KismetMathLibrary.FTrunc` (+ _returnvalue 1.0))) _returnvalue_3) (- _returnvalue _returnvalue_2)))))

(fn `UserConstructionScript`)