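; Game mode that runs a box-spawning game with score and error tracking, opening the end menu after more than four errors.
; BeginPlay finds all BP_Screen actors and, inside that screen loop, fills BoxObjects from the DT_BoxObjects data table.
; Tick uses a DoOnce and Delay cycle to periodically spawn BP_BoxBase, flagged Bad, using randomly indexed object class and score.
; AddScore and AddErrors update each screen, incrementing totals within that loop.
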(event `self.ReceiveBeginPlay`
  (bind _outactors (`GameplayStatics.GetAllActorsOfClass` "/Game/Blueprints/World/Screen/BP_Screen.BP_Screen_C"))
  (bind _output_get (set `self.Screen` _outactors))
  (for _array_element _output_get
    (`/Game/Blueprints/World/Screen/BP_Screen.UpdateScore` _array_element 0)
    (bind _outrownames (`DataTableFunctionLibrary.GetDataTableRowNames` "/Game/Blueprints/DT_BoxObjects.DT_BoxObjects"))
    (for _array_element_2 _outrownames
      (bind _returnvalue (`|GetDataTableRow` "/Game/Blueprints/DT_BoxObjects.DT_BoxObjects" _array_element_2)
        (:`then`
          (`KismetArrayLibrary.Array_Add` (`self.Box Objects`) _returnvalue))))))

(event `/Game/Blueprints/BPI_Main.AddScore`
  (params (ScoreToAdd :type Integer))
  (bind _returnvalue (+ (`self.Score`) ScoreToAdd))
  (for _array_element (`self.Screen`)
    (`/Game/Blueprints/World/Screen/BP_Screen.UpdateScore` _array_element _returnvalue)
    (set `self.Score` _returnvalue)))

(event `/Game/Blueprints/BPI_Main.Add Errors`
  (params (`Errors To Add` :type Integer))
  (bind _returnvalue (+ (`self.Errors`) `Errors To Add`))
  (for _array_element (`self.Screen`)
    (`/Game/Blueprints/BPI_Main.UpdateErrors` _array_element _returnvalue)
    (if (> _returnvalue 4)
      (`GameplayStatics.OpenLevelBySoftObjectPtr` "/Game/Levels/EndMenu.EndMenu")
      (else
        (set `self.Errors` _returnvalue)))))

(event `self.ReceiveTick`
  (params (DeltaSeconds :type "Float (single-precision)"))
  (bind _box_objects (`self.Box Objects`))
  (bind (_output_objectactorclass _output_score) (break `/Game/Blueprints/STRUCT_BoxObjectData` (`|GetArrayItem` _box_objects (`KismetMathLibrary.RandomIntegerInRange` 0 (- (`KismetArrayLibrary.Array_Length` _box_objects) 1)))))
  (`/Engine/EditorBlueprintResources/StandardMacros.DoOnce` false :!label _label
    (:`Completed`
      (`KismetSystemLibrary.Delay` 5.0)
      (`|SpawnActorFromClass` "/Game/Blueprints/World/Boxes/BP_BoxBase.BP_BoxBase_C" (`KismetMathLibrary.MakeTransform` (0.0 0.0 0.0)) "Undefined" "MultiplyWithRoot" null _output_objectactorclass _output_score true null)
      (goto _label :!via `Reset`))))

(fn `UserConstructionScript`)