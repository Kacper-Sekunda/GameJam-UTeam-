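; BP_Screen is an in-world screen that displays score and error values through a WB_Screen widget held by its Widget component.
; On BeginPlay it casts and caches that widget, then sets it back on the component.
; UpdateScore and UpdateErrors write their values into the cached widget when valid and print a debug "Hello".
; AddScore is an empty event.
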(event `self.ReceiveBeginPlay`
  (bind _widget (`self.Widget`))
  (bind _aswb_screen (cast `/Game/Blueprints/World/Screen/WB_Screen` (`WidgetComponent.GetWidget` _widget)))
  (bind _output_get (set `self.WidgetA` _aswb_screen))
  (`WidgetComponent.SetWidget` _widget _output_get))

(event `/Game/Blueprints/BPI_Main.UpdateScore`
  (params (Score :type Integer))
  (`/Engine/EditorBlueprintResources/StandardMacros.IsValid` (`self.WidgetA`)
    (:`Is Valid`
      (set `/Game/Blueprints/World/Screen/WB_Screen.Score` Score (`self.WidgetA`))
      (`KismetSystemLibrary.PrintString` "Hello"))))

(event `/Game/Blueprints/BPI_Main.UpdateErrors`
  (params (Errors :type Integer))
  (`/Engine/EditorBlueprintResources/StandardMacros.IsValid` (`self.WidgetA`)
    (:`Is Valid`
      (set `/Game/Blueprints/World/Screen/WB_Screen.Errors` Errors (`self.WidgetA`))
      (`KismetSystemLibrary.PrintString` "Hello"))))

(event `/Game/Blueprints/BPI_Main.AddScore`
  (params (ScoreToAdd :type Integer)))

(fn `UserConstructionScript`)