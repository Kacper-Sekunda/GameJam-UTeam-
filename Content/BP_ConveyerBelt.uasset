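; Conveyor belt Blueprint that exposes events for controlling its Speed variable.
; Events set Speed directly, add to it, or flip its sign to reverse it.
; DecreaseSpeed also adds its input, so it lowers Speed only when given a negative value.
; The graphs contain no movement or overlap logic; BeginPlay, overlap, Tick and the construction script are empty.
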(event `Set Speed`
  (params (`New Speed` :type "Float (double-precision)"))
  (set `self.Speed` `New Speed`))

(event `Increase Speed`
  (params (`Speed to Add` :type "Float (double-precision)"))
  (set `self.Speed` (+ (`self.Speed`) `Speed to Add`)))

(event `Decrease Speed`
  (params (`Speed to Minus` :type "Float (double-precision)"))
  (set `self.Speed` (+ (`self.Speed`) `Speed to Minus`)))

(event `Reverse Speed`
  (set `self.Speed` (* (`self.Speed`) -1.0)))

(fn `UserConstructionScript`)