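; BPC_MoveAlongConveyer is a component that carries its owning actor along a conveyer's spline.
; While active, Tick advances a stored distance by the conveyer's speed and delta time, then sets the owner's world transform at that spline distance, ignoring scale and without sweeping.
; TurnOn and TurnOff toggle the movement, and the distance is neither reset nor bounded here.
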(event `self.ReceiveTick`
  (params (DeltaSeconds :type "Float (single-precision)"))
  (if (`self.Active`)
    (bind _output_get (set `self.Current Position` (+ (`self.Current Position`) (* (`/Game/BP_ConveyerBelt.Speed` (`self.Conveyer`)) DeltaSeconds))))
    (`Actor.K2_SetActorTransform` (`self.GetOwner`) (`SplineComponent.GetTransformAtDistanceAlongSpline` (`/Game/BP_ConveyerBelt.Spline` (`self.Conveyer`)) _output_get "World" false) false false)))

(event `Turn On`
  (set `self.Active` true))

(event `Turn Off`
  (set `self.Active` false))