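; BP_Test is a test Blueprint that exercises the BPCCursorIcon component, which maps cursor icons to scene components.
; On BeginPlay it registers two icons, each with a placeholder sprite and the direct children of one of two scene components.
; Its FindIcon function passes a given component to BPCCursorIcon and returns the icon found for it.
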(event `self.ReceiveBeginPlay`
  (`/Game/Blueprints/Character/Cursor/BPC_CursorIcon.Create New Icon` (`self.BPC_CursorIcon`) "/Game/Blueprints/Character/Cursor/Untitled_Sprite.Untitled_Sprite" (`SceneComponent.GetChildrenComponents` (`self.Scene`) false))
  (`/Game/Blueprints/Character/Cursor/BPC_CursorIcon.Create New Icon` (`self.BPC_CursorIcon`) "/Game/Blueprints/Character/Cursor/Untitled1_Sprite.Untitled1_Sprite" (`SceneComponent.GetChildrenComponents` (`self.Scene1`) false)))

(fn `Find Icon`
  (params (Component :type "SceneComponent Object Reference"))
  (returns (Icon :type "PaperSprite Object Reference"))
  (bind _icon (`/Game/Blueprints/Character/Cursor/BPC_CursorIcon.Find Component Icon` (`self.BPC_CursorIcon`) Component))
  (return _icon))

(fn `UserConstructionScript`)