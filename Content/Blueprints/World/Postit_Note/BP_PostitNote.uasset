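; BP_PostitNote is a clickable post-it note that moves away and destroys itself when clicked.
; A construction-time material styles the Plane, which BPCCursorIcon registers with an arrow cursor icon at BeginPlay and exposes through FindIcon.
; Click plays a timeline that lerps the actor from its starting transform to TargetLocation, keeping the starting rotation, then destroys it on finish.
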(event `self.ReceiveBeginPlay`
  (bind (_target_location_location _target_location_rotation _target_location_scale) (`KismetMathLibrary.BreakTransform` (`self.Target Location`)))
  (`/Game/Blueprints/Character/Cursor/BPC_CursorIcon.Create New Icon` (`self.BPC_CursorIcon`) "/Game/Blueprints/Character/Cursor/Arrow_Sprite.Arrow_Sprite" (`|MakeArray` (`self.Plane`) :!type "SceneComponent Object Reference"))
  (bind _output_get (set `self.Base Location` (`self.GetTransform`)))
  (set `self.Target Location` (`KismetMathLibrary.MakeTransform` _target_location_location (.rotation _output_get) _target_location_scale)))

(event `/Game/Blueprints/Character/Cursor/BPI_Interaction.Click`
  (`KismetSystemLibrary.PrintString` "Note Move")
  (bind (_direction _newtrack_0) (`Timeline|Timeline` :!via `PlayFromStart`)
    (:`Update`
      (`self.K2_SetActorTransform` (`KismetMathLibrary.TLerp` (`self.Base Location`) (`self.Target Location`) _newtrack_0)))
    (:`Finished`
      (`self.K2_DestroyActor`))))

(fn `Find Icon`
  (params (Component :type "SceneComponent Object Reference"))
  (returns (Icon :type "PaperSprite Object Reference"))
  (bind _icon (`/Game/Blueprints/Character/Cursor/BPC_CursorIcon.Find Component Icon` (`self.BPC_CursorIcon`) Component))
  (return _icon))

(fn `UserConstructionScript`
  (`PrimitiveComponent.SetMaterial` (`self.Plane`) 0 (`self.Postit Material`)))