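; BP_Sucker is a world actor whose SUCKER component drops down, plays a suck-up effect and retracts when Deny is called.
; A timeline lowers it from the position cached at BeginPlay, then activates Suckup and ADA.
; After a short delay, a second timeline played in reverse lerps it from its current position toward the cached one and deactivates Suckup.
; The Sucking flag blocks retriggering until that finishes.
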(event `/Game/Blueprints/Character/Cursor/BPI_Interaction.Deny`
  (if (not (`self.Sucking`))
    (set `self.Sucking` true)
    (bind (_direction _alpha) (`Timeline|Timeline` :!via `PlayFromStart`)
      (:`Update`
        (`SceneComponent.K2_SetRelativeLocation` (`self.SUCKER`) (`KismetMathLibrary.VLerp` (`self.Relative Location`) (0.0 0.0 -195.0) _alpha) false false))
      (:`Finished`
        (`ActorComponent.Activate` (`self.Suckup`) false)
        (`ActorComponent.Activate` (`self.ADA`) false)
        (`KismetSystemLibrary.Delay` 1.1)
        (bind (_direction_2 _alpha_2) (`Timeline|Timeline_0` :!via `ReverseFromEnd`)
          (:`Update`
            (`SceneComponent.K2_SetRelativeLocation` (`self.SUCKER`) (`KismetMathLibrary.VLerp` (`SceneComponent.RelativeLocation` (`self.SUCKER`)) (`self.Relative Location`) _alpha_2) false false)
            (`ActorComponent.Deactivate` (`self.Suckup`)))
          (:`Finished`
            (set `self.Sucking` false)))))))

(event `self.ReceiveBeginPlay`
  (set `self.Relative Location` (`SceneComponent.RelativeLocation` (`self.SUCKER`))))

(fn `UserConstructionScript`)